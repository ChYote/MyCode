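; Interactive cube actor that toggles its rotation each time its Activate event is called.
; Activate flips ShouldRotate and uses it to select either a zero or a constant single-axis rate for the RotatingMovement component.
; The selection runs opposite to the flag's name: a true ShouldRotate picks the zero rate.
; Tick and the construction script only call their parents.
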(event EventBeginPlay
  (|CallParentFunction) ; This node is disabled and will not be called.\nDrag off pins to build functionality.
)

(event Collision|EventActorBeginOverlap
  (params (OtherActor :type Actor%20Object%20Reference))
  (|CallParentFunction OtherActor) ; This node is disabled and will not be called.\nDrag off pins to build functionality.
)

(event EventTick
  (params (DeltaSeconds :type Float%20%28single-precision%29))
  (|CallParentFunction DeltaSeconds))

(event EventActivate
  (Variables|Default|SetShouldRotate (not (Variables|Default|GetShouldRotate)))
  (Variables|/Script/Engine.RotatingMovementComponent|SetRotationRate (Variables|Default|GetRotatingMovement) (Math|Rotator|SelectRotator "0, 0, 0" "0,180.000000, 0" (Variables|Default|GetShouldRotate))))

(fn ConstructionScript
  (|CallParentFunction))