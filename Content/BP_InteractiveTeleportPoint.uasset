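; BP_InteractiveTeleportPoint is an interactive point that teleports the player pawn to its own location when activated.
; On BeginPlay it caches the first player pawn as a BP_PawnBase.
; The Activate event moves that pawn to a fixed height above the point's origin and keeps the pawn's current rotation.
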(event EventBeginPlay
  (|CallParentFunction)
  (bind _asbp_pawn_base (Utilities|Casting|CastToBP_PawnBase (Game|Player|GetPlayerPawn 0)))
  (Variables|Default|SetCurrentPlayer _asbp_pawn_base))

(event Collision|EventActorBeginOverlap
  (params (OtherActor :type Actor%20Object%20Reference))
  (|CallParentFunction OtherActor) ; This node is disabled and will not be called.\nDrag off pins to build functionality.
)

(event EventTick
  (params (DeltaSeconds :type Float%20%28single-precision%29))
  (|CallParentFunction DeltaSeconds) ; This node is disabled and will not be called.\nDrag off pins to build functionality.
)

(event EventActivate
  (bind _currentplayer (Variables|Default|GetCurrentPlayer))
  (Transformation|Teleport _currentplayer (+ (Transformation|GetActorLocation) "0, 0,180.000000") (Transformation|GetActorRotation _currentplayer)))

(fn ConstructionScript
  (|CallParentFunction))